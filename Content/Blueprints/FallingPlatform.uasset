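; Falling platform Blueprint that turns on physics for its platforms a set delay after something overlaps its Collision component.
; The construction script builds thin slabs as instances of one InstancedStaticMesh: one at the origin, then evenly spaced rows along local X and Y, sized by PlatformCount.
; Its nested loops fill only those two axes rather than a grid, stacking duplicate instances at each position.
; Physics is enabled on the whole instanced component, not per platform.
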(event OnComponentBeginOverlap(collision)
  (params (OverlappedComponent :type Primitive%20Component%20Object%20Reference) (OtherActor :type Actor%20Object%20Reference) (OtherComp :type Primitive%20Component%20Object%20Reference) (OtherBodyIndex :type Integer) (bFromSweep :type Boolean) (SweepResult :type Hit%20Result%20Structure%20%28by%20ref%29))
  (Utilities|FlowControl|Delay (Variables|Default|GetTime))
  (Physics|SetSimulatePhysics (Variables|Default|GetInstancedStaticMesh) true))

(fn ConstructionScript
  (Components|InstancedStaticMesh|AddInstance (Variables|Default|GetInstancedStaticMesh) (Math|Transform|MakeTransform "0, 0, 0" "0, 0, 0" "2.000000,2.000000,0.070000"))
  (for _index (range 1 (Variables|Default|GetPlatformCount))
    (for _index_2 (range 1 (Variables|Default|GetPlatformCount))
      (Components|InstancedStaticMesh|AddInstance (Variables|Default|GetInstancedStaticMesh) (Math|Transform|MakeTransform (Math|Vector|MakeVector (* _index_2 5e+02) 0.0 0.0) "0, 0, 0" "2.000000,2.000000,0.070000"))
      (Components|InstancedStaticMesh|AddInstance (Variables|Default|GetInstancedStaticMesh) (Math|Transform|MakeTransform (Math|Vector|MakeVector 0.0 (* _index 5e+02) 0.0) "0, 0, 0" "2.000000,2.000000,0.070000")))))