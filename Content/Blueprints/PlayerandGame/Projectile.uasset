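; Projectile actor that damages overlapping actors and can be hovered and destroyed through interaction.
; Overlap passes a DoOnce gate to apply damage and nudge a TopDownCharacter, resetting after a delay only when that cast succeeds.
; Cursor hover toggles a "selected" material parameter on the Projectile component, and the Interacted event destroys the actor.
; A physics impulse branch is present but disconnected.
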(event OnBeginCursorOver(Projectile)
  (params (TouchedComponent :type Primitive%20Component%20Object%20Reference))
  (Rendering|Material|SetScalarParameterValueonMaterials (Variables|Default|GetProjectile) "selected" 1.0))

(event OnEndCursorOver(Projectile)
  (params (TouchedComponent :type Primitive%20Component%20Object%20Reference))
  (Rendering|Material|SetScalarParameterValueonMaterials (Variables|Default|GetProjectile) "selected" 0.0))

(event EventInteracted
  (params (Player :type Top%20Down%20Character%20Object%20Reference))
  (Actor|DestroyActor))

(event Collision|EventActorBeginOverlap
  (params (OtherActor :type Actor%20Object%20Reference))
  (Utilities|FlowControl|DoOnce false :!label _label
    (:Completed
      (Game|Damage|ApplyDamage OtherActor 2e+01 0 0)
      (bind _astop_down_character (Utilities|Casting|CastToTopDownCharacter OtherActor))
      (Character|LaunchCharacter _astop_down_character "10.000000,10.000000, 0" false false)
      (Utilities|FlowControl|Delay 2.0)
      (goto _label Reset))))

(fn ConstructionScript)