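; AI enemy character that chases a perceived target and performs a leap attack, using a three-state machine run on Tick.
; AI Perception sets or clears the enemy, driving switches between idle, pursuing and attacking, with movement stopped outside pursuit.
; Within attack range it hops, lunges forward, then returns to idle.
; Overlapping actors take damage, and the top-down player character is knocked back, gated by a DoOnce cooldown.
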(event OnTargetPerceptionUpdated(AIPerception)
  (params (Actor :type Actor%20Object%20Reference) (Stimulus :type AI%20Stimulus%20Structure))
  (bind _bsuccessfullysensed (Utilities|Struct|BreakAIStimulus Stimulus))
  (Utilities|IsValid (Variables|Default|GetEnemy)
    (:Is%20Valid
      (if (and (== (Variables|Default|GetEnemy) Actor) (not _bsuccessfullysensed))
        (Variables|Default|SetEnemy 0)
        (CallFunction|StateSwitch "NewEnumerator0")))
    (:Is%20Not%20Valid
      (if _bsuccessfullysensed
        (Variables|Default|SetEnemy Actor)))))

(event EventTick
  (params (DeltaSeconds :type Float%20%28single-precision%29))
  (bind _enemy (Variables|Default|GetEnemy))
  (switch Utilities|FlowControl|Switch|SwitchonAI_States (Variables|Default|GetCurrentState)
    (:NewEnumerator0
      ;[1 1 1] Switch to Pursue if can see player
      (Utilities|IsValid (Variables|Default|GetEnemy)
        (:Is%20Valid
          (CallFunction|StateSwitch "NewEnumerator1"))))
    (:NewEnumerator1
      ;[1 1 1] Switch to Idle if can't see player
      (Utilities|IsValid _enemy
        (:Is%20Valid
          (AI|Navigation|SimpleMovetoLocation (Pawn|GetController) (Transformation|GetActorLocation _enemy))
          (bind _distancetoplayer (CallFunction|DistancetoPlayer))
          (if (< _distancetoplayer (Variables|Default|GetAttackDis))
            (CallFunction|StateSwitch "NewEnumerator2")))
        (:Is%20Not%20Valid
          (CallFunction|StateSwitch "NewEnumerator0"))))
    (:NewEnumerator2
      (Utilities|IsValid (Variables|Default|GetEnemy)
        (:Is%20Valid
          (Utilities|FlowControl|DoOnce false :!label _label
            (:Completed
              (Utilities|FlowControl|Delay 1.0)
              (Character|LaunchCharacter "0, 0,150.000000" false false)
              (Utilities|FlowControl|Delay 0.1)
              (Character|LaunchCharacter (* (Math|Vector|GetForwardVector (Transformation|GetActorRotation)) (Variables|Default|GetLeapDis)) false false)
              (CallFunction|StateSwitch "NewEnumerator0")
              (goto _label Reset))))))))

(event Collision|EventActorBeginOverlap
  (params (OtherActor :type Actor%20Object%20Reference))
  (Utilities|FlowControl|DoOnce false :!label _label
    (:Completed
      (Game|Damage|ApplyDamage OtherActor 2e+01 0 0)
      (bind _astop_down_character (Utilities|Casting|CastToTopDownCharacter OtherActor))
      (Character|LaunchCharacter _astop_down_character (* (Math|Vector|GetUnitDirection(Vector) (Transformation|GetWorldLocation (Variables|Default|GetCollider)) (Transformation|GetActorLocation _astop_down_character)) (Variables|Default|GetPushback)) false false)
      (Utilities|FlowControl|Delay 4.0)
      (goto _label Reset))))

(fn ConstructionScript)

(fn StateSwitch
  (params (Next%20State :type AI_States%20Enum :default "NewEnumerator0"))
  (bind _output_get (Variables|Default|SetCurrentState Next%20State))
  (switch Utilities|FlowControl|Switch|SwitchonAI_States _output_get
    (:NewEnumerator0
      _)
    (:NewEnumerator2
      _))
  (AI|Navigation|StopMovement (Pawn|GetController)))

(fn DistancetoPlayer
  (bind _returnvalue (Actor|GetActorOfClass "/Game/Blueprints/PlayerandGame/TopDownCharacter.TopDownCharacter_C"))
  (return (Math|Vector|VectorLength (- (Transformation|GetActorLocation _returnvalue) (Transformation|GetActorLocation)))))